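; BP_FlyUpArea is an updraft trigger volume that lifts the player character upward while inside its Box.
; A Player-tagged overlap starts a looping short-interval timer that runs Fly, and leaving the Box clears it.
; Fly sets the NeonTaoistCharacter to Falling and adds scaled Acceleration to its vertical velocity, capped at MaxSpeed, preserving horizontal velocity.
; A branch restoring Walking is unconnected and never runs.
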(event `self.Box.OnComponentBeginOverlap`
  (params (OverlappedComponent :type "PrimitiveComponent Object Reference") (OtherActor :type "Actor Object Reference") (OtherComp :type "PrimitiveComponent Object Reference") (OtherBodyIndex :type Integer) (bFromSweep :type Boolean) (SweepResult :type "HitResult Structure (by ref)"))
  (if (`self.ActorHasTag` OtherActor "Player")
    (bind _returnvalue (`KismetSystemLibrary.K2_SetTimerDelegate` (delegate `Fly`) 0.01 true 0.01))))

(event `Fly`
  (bind _asneon_taoist_character (cast `NeonTaoistCharacter` (stale `self.Box.OnComponentBeginOverlap` OtherActor)))
  (bind _charactermovement (`Character.CharacterMovement` _asneon_taoist_character))
  (`CharacterMovementComponent.SetMovementMode` _charactermovement "MOVE_Falling" 0)
  (bind (_velocity_x _velocity_y _velocity_z) (`KismetMathLibrary.BreakVector` (`MovementComponent.Velocity` _charactermovement)))
  (set `MovementComponent.Velocity` (`KismetMathLibrary.MakeVector` _velocity_x _velocity_y (`KismetMathLibrary.FMin` (+ _velocity_z (/ (`self.Acceleration`) 20.0)) (`self.MaxSpeed`))) _charactermovement))

(event `self.Box.OnComponentEndOverlap`
  (params (OverlappedComponent :type "PrimitiveComponent Object Reference") (OtherActor :type "Actor Object Reference") (OtherComp :type "PrimitiveComponent Object Reference") (OtherBodyIndex :type Integer))
  (if (`self.ActorHasTag` OtherActor "Player")
    (`KismetSystemLibrary.K2_ClearAndInvalidateTimerHandle` (stale `self.Box.OnComponentBeginOverlap` _returnvalue))))

(fn `UserConstructionScript`)