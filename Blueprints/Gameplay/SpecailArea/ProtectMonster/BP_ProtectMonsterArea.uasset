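; BP_ProtectMonsterArea is a protector actor that links to nearby NeonTaoist monsters, buffs them, and kills them when it is destroyed.
; One second after BeginPlay, it captures monsters overlapping its box once, then disables the box's collision.
; Each gets a Niagara beam, with endpoints set once, and the GE_WhosYourDaddy gameplay effect through the ability system.
; Its OnDestroyed handler calls Die on every captured monster.
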(event `self.ReceiveBeginPlay`
  (`|ExecutionSequence`
    (:`then_0`
      (`KismetSystemLibrary.Delay` 1.0)
      (`self.GetNearestMonster`)
      (for _array_element (`self.Monsters`)
        (`|ExecutionSequence`
          (:`then_0`
            (bind _returnvalue (`AddComponent|NODE_AddNiagaraComponent-0`))
            (`NiagaraComponent.SetVariableVec3` _returnvalue "BeamStart" (`self.K2_GetActorLocation`))
            (`NiagaraComponent.SetVariableVec3` _returnvalue "BeamEnd" (`self.K2_GetActorLocation` _array_element)))
          (:`then_1`
            (bind _asneon_taoist_monster_base (cast `NeonTaoistMonsterBase` _array_element))
            (`AbilitySystemComponent.BP_ApplyGameplayEffectToTarget` :`self` (`self.AbilitySystem`) :`GameplayEffectClass` "/Game/ThirdPerson/Blueprints/Gameplay/SpecailArea/ProtectMonster/GE_WhosYourDaddy.GE_WhosYourDaddy_C" :`Target` (`AbilitySystemBlueprintLibrary.GetAbilitySystemComponent` _asneon_taoist_monster_base))))))
    (:`then_1`
      (add `self.OnDestroyed` (delegate `OnDestroyed_Event`)))))

(event `OnDestroyed_Event` :!signature `self.OnDestroyed`
  (params (DestroyedActor :type "Actor Object Reference"))
  (for _array_element (`self.Monsters`)
    (bind _asneon_taoist_monster_base (cast `NeonTaoistMonsterBase` _array_element))
    (`NeonTaoistMonsterBase.Die` _asneon_taoist_monster_base)))

(fn `GetNearestMonster`
  (bind _outactors (`KismetSystemLibrary.ComponentOverlapActors` (`self.BoxComponent`) (`SceneComponent.K2_GetComponentToWorld` (`self.BoxComponent`)) (`self.Object Types`) "/Script/NeonTaoist.NeonTaoistMonsterBase"))
  (set `self.Monsters` _outactors)
  (`PrimitiveComponent.SetCollisionEnabled` (`self.BoxComponent`) "NoCollision"))

(fn `UserConstructionScript`)