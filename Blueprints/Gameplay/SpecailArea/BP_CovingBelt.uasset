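; BP_CovingBelt is a conveyor belt area that carries characters along the direction of its mesh.
; Each Tick it finds BP_Character actors overlapping its Box and moves them with a swept world offset along the StaticMesh forward vector, scaled by Speed and frame time.
; Any begin-overlap on the Box plays a 2D conveyor sound.
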(event `self.Box.OnComponentBeginOverlap`
  (params (OverlappedComponent :type "PrimitiveComponent Object Reference") (OtherActor :type "Actor Object Reference") (OtherComp :type "PrimitiveComponent Object Reference") (OtherBodyIndex :type Integer) (bFromSweep :type Boolean) (SweepResult :type "HitResult Structure (by ref)"))
  (`GameplayStatics.PlaySound2D` "/Game/AudioResource/Sounds/Map/Sound_CovingBelt.Sound_CovingBelt" 1.0 1.0 0.0 null null))

(event `self.ReceiveTick`
  (params (DeltaSeconds :type "Float (single-precision)"))
  (for _array_element (`PrimitiveComponent.GetOverlappingActors` (`self.Box`) "/Game/Art/Frank_Platformer1/Animations/BP_Character.BP_Character_C")
    (`self.K2_AddActorWorldOffset` _array_element (* (`KismetMathLibrary.GetForwardVector` (`SceneComponent.K2_GetComponentRotation` (`self.StaticMesh`))) (* DeltaSeconds (`self.Speed`))) true false)))

(fn `UserConstructionScript`)