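; Trigger actor that ends the level in victory when a player-tagged actor overlaps it with no monsters left.
; The monster count comes from NeonTaoistGameState; at zero it disables player input, plays victory music, sets IsWin and shows the WBP_GameFail widget, despite that widget's name.
; Otherwise it shows a WBP_CommonTextNotice saying the monsters are not all eliminated.
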(event `self.ReceiveActorBeginOverlap`
  (params (OtherActor :type "Actor Object Reference"))
  (if (`self.ActorHasTag` OtherActor "Player")
    (bind _asneon_taoist_game_state (cast `NeonTaoistGameState` (`GameplayStatics.GetGameState`)))
    (if (== (`NeonTaoistGameState.GetMonsterCount` _asneon_taoist_game_state) 0)
      (`self.DisableInput` (`GameplayStatics.GetPlayerCharacter` 0) (`GameplayStatics.GetPlayerController` 0))
      (`GameplayStatics.PlaySound2D` "/Game/AudioResource/BGM/Victory/BGM_Vic.BGM_Vic" 1.0 1.0 0.0 null null)
      (set `self.IsWin` true)
      (bind _returnvalue (`|CreateWidget` "/Game/ThirdPerson/UI/AroundGame/WBP_GameFail.WBP_GameFail_C"))
      (`UserWidget.AddToViewport` _returnvalue 0)
      (else
        (bind _returnvalue_2 (`|CreateWidget` "/Game/ThirdPerson/UI/Common/WBP_CommonTextNotice.WBP_CommonTextNotice_C"))
        (`/Game/ThirdPerson/UI/Common/WBP_CommonTextNotice.InitialText` _returnvalue_2 "怪物未被全部消灭！")
        (`UserWidget.AddToViewport` _returnvalue_2 0)))))

(fn `UserConstructionScript`)