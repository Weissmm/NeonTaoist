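; BP_CanClimbWall is a climbable wall zone that toggles the player character's climbing state through a Box overlap volume.
; On entry, it sets IsClimbing on the BP_Character anim instance, switches movement to Flying and sets a slight downward velocity once.
; On exit, it clears the flag and restores Walking.
; It responds only to player 0's character and contains no climb input logic.
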(event `self.Box.OnComponentBeginOverlap`
  (params (OverlappedComponent :type "PrimitiveComponent Object Reference") (OtherActor :type "Actor Object Reference") (OtherComp :type "PrimitiveComponent Object Reference") (OtherBodyIndex :type Integer) (bFromSweep :type Boolean) (SweepResult :type "HitResult Structure (by ref)"))
  (bind _returnvalue (`GameplayStatics.GetPlayerCharacter` 0))
  (bind _charactermovement (`Character.CharacterMovement` _returnvalue))
  (if (== OtherActor _returnvalue)
    (`|ExecutionSequence`
      (:`then_0`
        (bind _asbp_character (cast `/Game/Art/Frank_Platformer1/Animations/BP_Character` _returnvalue))
        (set `NeonTaoistAnimInstance.bIsClimbing` true (`NeonTaoistCharacter.AnimInstance` _asbp_character)))
      (:`then_1`
        (`CharacterMovementComponent.SetMovementMode` _charactermovement "MOVE_Flying" 0))
      (:`then_2`
        (set `MovementComponent.Velocity` (0.0 0.0 -60.0) _charactermovement)))))

(event `self.Box.OnComponentEndOverlap`
  (params (OverlappedComponent :type "PrimitiveComponent Object Reference") (OtherActor :type "Actor Object Reference") (OtherComp :type "PrimitiveComponent Object Reference") (OtherBodyIndex :type Integer))
  (bind _returnvalue (`GameplayStatics.GetPlayerCharacter` 0))
  (if (== OtherActor _returnvalue)
    (`|ExecutionSequence`
      (:`then_0`
        (bind _asbp_character (cast `/Game/Art/Frank_Platformer1/Animations/BP_Character` _returnvalue))
        (set `NeonTaoistAnimInstance.bIsClimbing` false (`NeonTaoistCharacter.AnimInstance` _asbp_character)))
      (:`then_1`
        (`CharacterMovementComponent.SetMovementMode` (`Character.CharacterMovement` _returnvalue) "MOVE_Walking" 0)))))

(fn `UserConstructionScript`
  (`parent.UserConstructionScript`))