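; BP_FadeWall is a wall actor that removes itself after the player touches its trigger box.
; An overlap with an actor tagged "Player" starts a one-second delay, then the wall destroys itself and plays the fade-wall sound in 2D.
; Despite the name, the graph has no visual fade, and the sound call comes after the destroy call.
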(event `self.Box.OnComponentBeginOverlap`
  (params (OverlappedComponent :type "PrimitiveComponent Object Reference") (OtherActor :type "Actor Object Reference") (OtherComp :type "PrimitiveComponent Object Reference") (OtherBodyIndex :type Integer) (bFromSweep :type Boolean) (SweepResult :type "HitResult Structure (by ref)"))
  (if (`self.ActorHasTag` OtherActor "Player")
    (`KismetSystemLibrary.Delay` 1.0)
    (`self.K2_DestroyActor`)
    (`GameplayStatics.PlaySound2D` "/Game/AudioResource/Sounds/Map/Sound_Fadewall.Sound_Fadewall" 1.0 1.0 0.0 null null)))

(fn `UserConstructionScript`
  (`parent.UserConstructionScript`))