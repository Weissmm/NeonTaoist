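; Corner trigger actor that turns the player between X and Y movement axes in a plane-constrained, side-on movement setup.
; On player overlap it snaps the capsule to the actor's XY, rotates it, switches the movement plane constraint and updates the character's direction flags.
; Tick then lerps the camera boom yaw to face opposite the new heading, using AdjustInput to take the shortest way around the 360-degree wrap.
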(event `self.ReceiveTick`
  (params (DeltaSeconds :type "Float (single-precision)"))
  (if (`self.bTurnning`)
    (if (`self.bTurnToX`)
      (`self.Turning` DeltaSeconds (`self.XtoYRotation`))
      (else
        (`self.Turning` DeltaSeconds (`self.YtoXRotation`))))))

(event `self.CharacterBox.OnComponentBeginOverlap`
  (params (OverlappedComponent :type "PrimitiveComponent Object Reference") (OtherActor :type "Actor Object Reference") (OtherComp :type "PrimitiveComponent Object Reference") (OtherBodyIndex :type Integer) (bFromSweep :type Boolean) (SweepResult :type "HitResult Structure (by ref)"))
  (bind _returnvalue (`GameplayStatics.GetPlayerPawn` 0))
  (if (== OtherActor _returnvalue)
    (set `self.bTurnning` true)
    (bind _asbp_third_person_character (cast `/Game/ThirdPerson/Blueprints/BP_ThirdPersonCharacter` _returnvalue))
    (bind _output_get (set `self.RotationBegin` (`SpringArmComponent.GetTargetRotation` (`NeonTaoistCharacter.CameraBoom` _asbp_third_person_character))))
    (`KismetSystemLibrary.PrintString` (`KismetStringLibrary.Conv_RotatorToString` _output_get))
    (bind _capsulecomponent (`Character.CapsuleComponent` _asbp_third_person_character))
    (`SceneComponent.K2_SetWorldLocation` _capsulecomponent (`KismetMathLibrary.MakeVector` (.x (`self.K2_GetActorLocation`)) (.y (`self.K2_GetActorLocation`)) (.z (`SceneComponent.K2_GetComponentLocation` _capsulecomponent))) false false)
    (if (`NeonTaoistCharacter.bMovingOnX` _asbp_third_person_character)
      (`SceneComponent.K2_SetWorldRotation` _capsulecomponent (`self.XtoYRotation`) false false)
      (bind _charactermovement (`Character.CharacterMovement` _asbp_third_person_character))
      (`MovementComponent.SetPlaneConstraintAxisSetting` _charactermovement "Y")
      (set `NeonTaoistCharacter.bMovingOnX` false _asbp_third_person_character)
      (set `self.bTurnToX` false)
      (set `NeonTaoistCharacter.bMovingOnYR` (`self.isMovingOnYR`) _asbp_third_person_character)
      (else
        (`SceneComponent.K2_SetWorldRotation` _capsulecomponent (`self.YtoXRotation`) false false)
        (`MovementComponent.SetPlaneConstraintAxisSetting` _charactermovement "X")
        (set `NeonTaoistCharacter.bMovingOnX` true _asbp_third_person_character)
        (set `self.bTurnToX` true)
        (set `NeonTaoistCharacter.bMovingOnXR` (`self.isMovingOnXR`) _asbp_third_person_character)))))

(fn `Adjust Input`
  (params (begin :type "Rotator Structure") (Target :type "Rotator Structure"))
  (returns (adjustedbegin :type "Rotator Structure") (adjustedTarget :type "Rotator Structure"))
  (bind _yaw (.yaw begin))
  (bind _yaw_2 (.yaw Target))
  (if (> (`KismetMathLibrary.Abs` (- _yaw _yaw_2)) 180.0)
    (if (> _yaw _yaw_2)
      (return (`KismetMathLibrary.MakeRotator` 0.0 0.0 (- _yaw 360.0)) (`local.Target`))
      (else
        (return (`local.begin`) (`KismetMathLibrary.MakeRotator` 0.0 0.0 (- _yaw_2 360.0)))))
    (else
      (return (`local.begin`) (`local.Target`)))))

(fn `Turning`
  (params (DeltaTime :type "Float (double-precision)") (Rotation :type "Rotator Structure"))
  (locals (Character :type "/Game/ThirdPerson/Blueprints/BP_ThirdPersonCharacter Object Reference") (Rotator :type "Rotator Structure"))
  (bind (_adjustedbegin _adjustedtarget) (`self.Adjust Input` (`self.RotationBegin`) (`KismetMathLibrary.MakeRotator` 0.0 0.0 (mod (+ 180.0 (.yaw (`local.Rotator`))) 360.0))))
  (set `local.Rotator` Rotation)
  (bind _output_get (set `self.LerpValue` (+ (`self.LerpValue`) (* DeltaTime 1.0))))
  (bind _asbp_third_person_character (cast `/Game/ThirdPerson/Blueprints/BP_ThirdPersonCharacter` (`GameplayStatics.GetPlayerPawn` 0)))
  (bind _output_get_2 (set `local.Character` _asbp_third_person_character))
  (bind _returnvalue (`KismetMathLibrary.RLerp` _adjustedbegin _adjustedtarget (`KismetMathLibrary.FClamp` _output_get)))
  (`SceneComponent.K2_SetWorldRotation` (`NeonTaoistCharacter.CameraBoom` _output_get_2) _returnvalue false false)
  (if (<= (`KismetMathLibrary.Abs` (- (.yaw _returnvalue) (.yaw _adjustedtarget))) 0.1)
    (set `self.LerpValue` 0.0)
    (set `self.bTurnning` false)))

(fn `UserConstructionScript`)