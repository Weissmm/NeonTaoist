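; BP_JumpCard is a card pickup that grants the player a jump card.
; GetCard casts the player pawn to BP_ThirdPersonCharacter and asks its BPCCharacterCardList component whether a jump card is collectable.
; If so, it collects the card there, calls GetCardFinished and plays a 2D pickup sound.
; The event graph holds only disabled default events, so all of its own logic lives in GetCard.
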(fn `GetCard`
  (bind _asbp_third_person_character (cast `/Game/ThirdPerson/Blueprints/BP_ThirdPersonCharacter` (`GameplayStatics.GetPlayerPawn` 0)))
  (bind _bpc_charactercardlist (`/Game/ThirdPerson/Blueprints/BP_ThirdPersonCharacter.BPC_CharacterCardList` _asbp_third_person_character))
  (if (`/Game/ThirdPerson/Blueprints/Characters/BPC_CharacterCardList.isJumpCardCollectable` _bpc_charactercardlist)
    (`/Game/ThirdPerson/Blueprints/Characters/BPC_CharacterCardList.CollectJumpCard` _bpc_charactercardlist)
    (`self.GetCardFinished`)
    (`GameplayStatics.PlaySound2D` "/Game/AudioResource/Sounds/Card/Sound_Getcard.Sound_Getcard" 1.0 1.0 0.0 null null)))

(fn `UserConstructionScript`
  (`parent.UserConstructionScript`))