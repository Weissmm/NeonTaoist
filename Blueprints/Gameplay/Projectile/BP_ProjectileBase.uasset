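; Base projectile Blueprint that launches along a forward direction derived from player pawn 0 when play begins.
; Init sets the ProjectileMovement velocity to that direction scaled by Speed, regardless of who spawned the projectile.
; SafeDestory retires it without immediate destruction: it disables sphere collision, toggles visibility down the component tree, deactivates movement and sets a lifespan from the given delay.
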(event `self.ReceiveBeginPlay`
  (`self.Init`))

(fn `Init`
  (bind _returnvalue (`NeonTaoistAbilityCommon.GetForwardDirection` (`GameplayStatics.GetPlayerPawn` 0)))
  (set `MovementComponent.Velocity` (* _returnvalue (`self.Speed`)) (`self.ProjectileMovement`)))

(fn `SafeDestory`
  (params (Delay :type "Float (double-precision)" :default 0.1))
  (`self.SetLifeSpan` Delay)
  (`PrimitiveComponent.SetCollisionEnabled` (`self.Sphere`) "NoCollision")
  (`SceneComponent.ToggleVisibility` (`self.DefaultSceneRoot`) true)
  (`ActorComponent.Deactivate` (`self.ProjectileMovement`)))

(fn `UserConstructionScript`)