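; Bomb projectile that explodes on overlapping anything not tagged MonsterProjectile, with particles, sound and delayed self-destruction.
; Explode range-queries to apply GE_DealDamage to monsters and remove destructible or fade walls.
; PlayerMove, called twice per blast, adds velocity pulling a nearby player toward the bomb, switching to Falling if vertical.
; Timers and offsets jolt the side-view camera and FOV; an interpolated player move is left unconnected.
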(event `self.ReceiveBeginPlay`
  (`self.SetActorTickEnabled` false))

(event `self.ReceiveTick`
  (params (DeltaSeconds :type "Float (single-precision)")))

(event `self.Sphere.OnComponentBeginOverlap`
  (params (OverlappedComponent :type "PrimitiveComponent Object Reference") (OtherActor :type "Actor Object Reference") (OtherComp :type "PrimitiveComponent Object Reference") (OtherBodyIndex :type Integer) (bFromSweep :type Boolean) (SweepResult :type "HitResult Structure (by ref)"))
  (if (not (`self.ActorHasTag` OtherActor "MonsterProjectile"))
    (`GameplayStatics.SpawnEmitterAtLocation` "/Game/VFX_Pack/Particles/P_Mid_Explosion.P_Mid_Explosion" (`self.K2_GetActorLocation`) (struct) (`self.Scale`))
    (`self.Explode`)
    (`GameplayStatics.PlaySound2D` "/Engine/EditorSounds/GamePreview/EndSimulate.EndSimulate" 1.0 1.0 0.0 null null)
    (`self.PlayerMove`)
    (`|ExecutionSequence`
      (:`then_0`
        (`self.SetActorTickEnabled` false)
        (`self.SafeDestory` 0.17))
      (:`then_1`
        (bind _asbp_third_person_character (cast `/Game/ThirdPerson/Blueprints/BP_ThirdPersonCharacter` (`GameplayStatics.GetPlayerPawn` 0)))
        (`|ExecutionSequence`
          (:`then_0`
            (bind _sideviewcameracomponent (`NeonTaoistCharacter.SideViewCameraComponent` _asbp_third_person_character))
            (`SceneComponent.K2_AddWorldOffset` _sideviewcameracomponent (-10.0 10.0 10.0) false false)
            (`KismetSystemLibrary.Delay` 0.06)
            (`SceneComponent.K2_AddWorldOffset` _sideviewcameracomponent (10.0 -10.0 -10.0) false false))
          (:`then_1`
            (`KismetSystemLibrary.K2_SetTimerDelegate` (delegate `SetCameraScale`) 0.02 true)
            (`KismetSystemLibrary.Delay` 0.05)
            (`KismetSystemLibrary.K2_SetTimerDelegate` (delegate `SetCameraScale1`) 0.02 true)
            (`KismetSystemLibrary.Delay` 0.05))
          (:`then_2`
            (`self.PlayerMove`)))))))

(event `SetCameraScale`
  (set `self.CameraAlpha` (`KismetMathLibrary.FClamp` (+ (`self.CameraAlpha`) 0.4)))
  (`CameraComponent.SetFieldOfView` (`NeonTaoistCharacter.SideViewCameraComponent` (stale `self.Sphere.OnComponentBeginOverlap` _asbp_third_person_character)) (`KismetMathLibrary.Lerp` 100.0 99.0 (`self.CameraAlpha`))))

(event `SetCameraScale1`
  (set `self.CameraAlpha` (`KismetMathLibrary.FClamp` (+ (`self.CameraAlpha`) 0.4)))
  (`CameraComponent.SetFieldOfView` (`NeonTaoistCharacter.SideViewCameraComponent` (stale `self.Sphere.OnComponentBeginOverlap` _asbp_third_person_character)) (`KismetMathLibrary.Lerp` 99.0 100.0 (`self.CameraAlpha`))))

(fn `Explode`
  (bind _overlapactors (`NeonTaoistAbilityCommon.OverlapRangeQuery` self (`self.ExplodeRange`) "PlayerAttack"))
  (for _array_element _overlapactors
    (if (`self.ActorHasTag` _array_element "Monster")
      (`NeonTaoistAbilityCommon.ApplyGEToTargetWithCallerData` (`GameplayStatics.GetPlayerPawn` 0) _array_element "/Game/ThirdPerson/Blueprints/Abilities/Character/GE_DealDamage.GE_DealDamage_C" (struct :`TagName` "GE.DamageMagnitude") (`self.Damage`))
      (elif (or (`self.ActorHasTag` _array_element "CanBeDestroyedWall") (`self.ActorHasTag` _array_element "FadeWall"))
        (`self.SetLifeSpan` _array_element 0.01))))
  (return))

(fn `GetMoveDirection`
  (set `self.MoveDirection` (`KismetMathLibrary.Normal` (- (`self.K2_GetActorLocation`) (`self.K2_GetActorLocation` (`GameplayStatics.GetPlayerCharacter` 0))))))

(fn `GetTargetLocation`
  (bind _returnvalue (`self.K2_GetActorLocation` (`GameplayStatics.GetPlayerCharacter` 0)))
  (set `self.TargetLocation` (+ _returnvalue (* (`KismetMathLibrary.Normal` (- (`self.K2_GetActorLocation`) _returnvalue)) (`self.MoveDistance`))))
  (return))

(fn `PlayerMove`
  (bind _movedirection (`self.MoveDirection`))
  (bind _overlapactors (`NeonTaoistAbilityCommon.OverlapRangeQuery` self (`self.PlayerRange`) "OverlapOnlyPawn"))
  (for _array_element _overlapactors
    (if (`self.ActorHasTag` _array_element "Player")
      (`self.GetTargetLocation`)
      (set `self.bMoved` true)
      (bind _asneon_taoist_character (cast `NeonTaoistCharacter` (`GameplayStatics.GetPlayerPawn` 0)))
      (`self.GetMoveDirection`)
      (if (!= (.z _movedirection) 0.0)
        (bind _charactermovement (`Character.CharacterMovement` _asneon_taoist_character))
        (`CharacterMovementComponent.SetMovementMode` _charactermovement "MOVE_Falling" 0))
      (set `MovementComponent.Velocity` (+ (`MovementComponent.Velocity` _charactermovement) (* _movedirection (`self.MoveSpeed`))) _charactermovement)
      (return))))

(fn `UserConstructionScript`
  (`parent.UserConstructionScript`))