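; Main menu camera actor that glides between root, character select and level select viewpoints.
; Begin functions set the start pose and a turning flag, which Tick uses to lerp the scene root's location and rotation to the target transform, then update the current-screen flags.
; Back steps to the previous screen.
; BeginArena looks unfinished: it applies a single lerp toward the arena transform without advancing and has no Tick branch.
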(event `self.ReceiveTick`
  (params (DeltaSeconds :type "Float (single-precision)"))
  (if (`self.bTurningToSelectCharacter`)
    (`self.ToSecectCharacter` DeltaSeconds)
    (elif (`self.bTurningToSelectLevel`)
      (`self.ToSecectLevel` DeltaSeconds)
      (elif (`self.bTurningToRoot`)
        (`self.ToRoot` DeltaSeconds)))))

(fn `Back`
  (if (`self.bSelectCharacter`)
    (`self.BeginRoot`)
    (else
      (`self.BeginSelectCharacter`))))

(fn `BeginArena`
  (bind (_selectarenatransform_location _selectarenatransform_rotation) (`KismetMathLibrary.BreakTransform` (`self.SelectArenaTransform`)))
  (bind _output_get (set `self.LerpValue` (+ (`self.LerpValue`) (* 0.0 0.75))))
  (bind _returnvalue (`KismetMathLibrary.FClamp` _output_get))
  (`SceneComponent.K2_SetWorldRotation` (`self.DefaultSceneRoot`) (`KismetMathLibrary.RLerp` (`self.BeginRotation`) _selectarenatransform_rotation _returnvalue) false false)
  (`SceneComponent.K2_SetWorldLocation` (`self.DefaultSceneRoot`) (`KismetMathLibrary.VLerp` (`self.BeginLocation`) _selectarenatransform_location _returnvalue) false false))

(fn `BeginRoot`
  (bind (_selectcharactertransform_location _selectcharactertransform_rotation) (`KismetMathLibrary.BreakTransform` (`self.SelectCharacterTransform`)))
  (set `self.bTurningToRoot` true)
  (set `self.BeginRotation` _selectcharactertransform_rotation)
  (set `self.BeginLocation` _selectcharactertransform_location))

(fn `BeginSelectCharacter`
  (bind (_selectleveltransform_location _selectleveltransform_rotation) (`KismetMathLibrary.BreakTransform` (`self.SelectLevelTransform`)))
  (bind (_roottransform_location _roottransform_rotation) (`KismetMathLibrary.BreakTransform` (`self.RootTransform`)))
  (set `self.bTurningToSelectCharacter` true)
  (if (`self.bInRoot`)
    (set `self.BeginLocation` _roottransform_location)
    (set `self.BeginRotation` _roottransform_rotation)
    (else
      (set `self.BeginLocation` _selectleveltransform_location)
      (set `self.BeginRotation` _selectleveltransform_rotation))))

(fn `BeginSelectLevel`
  (bind (_selectcharactertransform_location _selectcharactertransform_rotation) (`KismetMathLibrary.BreakTransform` (`self.SelectCharacterTransform`)))
  (set `self.BeginLocation` _selectcharactertransform_location)
  (set `self.BeginRotation` _selectcharactertransform_rotation)
  (set `self.bTurningToSelectLevel` true))

(fn `ToRoot`
  (params (DeltaTime :type "Float (double-precision)"))
  (bind (_roottransform_location _roottransform_rotation) (`KismetMathLibrary.BreakTransform` (`self.RootTransform`)))
  (bind _output_get (set `self.LerpValue` (+ (`self.LerpValue`) (* DeltaTime 0.75))))
  (bind _returnvalue (`KismetMathLibrary.FClamp` _output_get))
  (`SceneComponent.K2_SetWorldRotation` (`self.DefaultSceneRoot`) (`KismetMathLibrary.RLerp` (`self.BeginRotation`) _roottransform_rotation _returnvalue) false false)
  (`SceneComponent.K2_SetWorldLocation` (`self.DefaultSceneRoot`) (`KismetMathLibrary.VLerp` (`self.BeginLocation`) _roottransform_location _returnvalue) false false)
  (if (== _returnvalue 1.0)
    (set `self.bTurningToRoot` false)
    (set `self.bInRoot` true)
    (set `self.bSelectCharacter` false)
    (set `self.bSelectLevel` false)
    (set `self.LerpValue` 0.0)))

(fn `ToSecectCharacter`
  (params (DeltaTime :type "Float (double-precision)"))
  (bind (_selectcharactertransform_location _selectcharactertransform_rotation) (`KismetMathLibrary.BreakTransform` (`self.SelectCharacterTransform`)))
  (bind _output_get (set `self.LerpValue` (+ (`self.LerpValue`) (* DeltaTime 0.75))))
  (bind _returnvalue (`KismetMathLibrary.FClamp` _output_get))
  (`SceneComponent.K2_SetWorldRotation` (`self.DefaultSceneRoot`) (`KismetMathLibrary.RLerp` (`self.BeginRotation`) _selectcharactertransform_rotation _returnvalue) false false)
  (`SceneComponent.K2_SetWorldLocation` (`self.DefaultSceneRoot`) (`KismetMathLibrary.VLerp` (`self.BeginLocation`) _selectcharactertransform_location _returnvalue) false false)
  (if (== _returnvalue 1.0)
    (set `self.bTurningToSelectCharacter` false)
    (set `self.bInRoot` false)
    (set `self.bSelectCharacter` true)
    (set `self.bSelectLevel` false)
    (set `self.LerpValue` 0.0)))

(fn `ToSecectLevel`
  (params (DeltaTime :type "Float (double-precision)"))
  (bind (_selectleveltransform_location _selectleveltransform_rotation) (`KismetMathLibrary.BreakTransform` (`self.SelectLevelTransform`)))
  (bind _output_get (set `self.LerpValue` (+ (`self.LerpValue`) (* DeltaTime 0.75))))
  (bind _returnvalue (`KismetMathLibrary.FClamp` _output_get))
  (`SceneComponent.K2_SetWorldRotation` (`self.DefaultSceneRoot`) (`KismetMathLibrary.RLerp` (`self.BeginRotation`) _selectleveltransform_rotation _returnvalue) false false)
  (`SceneComponent.K2_SetWorldLocation` (`self.DefaultSceneRoot`) (`KismetMathLibrary.VLerp` (`self.BeginLocation`) _selectleveltransform_location _returnvalue) false false)
  (if (== _returnvalue 1.0)
    (set `self.bTurningToSelectLevel` false)
    (set `self.bInRoot` false)
    (set `self.bSelectLevel` true)
    (set `self.bSelectCharacter` false)
    (set `self.LerpValue` 0.0)))

(fn `UserConstructionScript`)