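; Character card inventory that tracks Jump, Boom and Sprint card stacks across two ability slots.
; Collecting cards claims a free slot and adds handgun ammo, rifle ammo or shield time respectively, with collectable checks limiting pickups.
; Click spends a round or toggles the shield timer drained on Tick, while Slide spends a card.
; Card counts follow ammo and shield use, emptied stacks free their slot, and CallCardChangeEvent signals changes.
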(event `self.ReceiveTick`
  (params (DeltaSeconds :type "Float (single-precision)"))
  (if (`self.bShieldOpen`)
    (bind _output_get (set `self.ShieldTime` (- (`self.ShieldTime`) DeltaSeconds)))
    (bind _returnvalue (`KismetMathLibrary.FFloor` (* _output_get 10.0)))
    (if (== (mod _returnvalue 10) 0)
      (bind _output_get_2 (set `self.sprintCardNum` (/ _returnvalue 10)))
      (if (== _output_get_2 0)
        (set `self.bShieldOpen` false)
        (if (`|EnumEquality` (`self.Card1`) "NewEnumerator2")
          (set `self.isAbility1Free` true)
          (else
            (set `self.isAbility2Free` true))))
      (`self.CardChangeEvent`))))

(fn `ClickBoomCard`
  (bind _output_get (set `self.rifleGunAmmo` (- (`self.rifleGunAmmo`) 1)))
  (if (== (mod _output_get (`self.rifleGunAmmoPerCard`)) 0)
    (bind _output_get_2 (set `self.boomCardNum` (- (`self.boomCardNum`) 1)))
    (if (== _output_get_2 0)
      (if (`|EnumEquality` (`self.Card1`) "NewEnumerator1")
        (set `self.isAbility1Free` true)
        (else
          (set `self.isAbility2Free` true)))
      (`self.CardChangeEvent`))))

(fn `ClickJumpCard`
  (bind _output_get (set `self.handGunAmmo` (- (`self.handGunAmmo`) 1)))
  (if (== (mod _output_get (`self.handGunAmmoPerCard`)) 0)
    (bind _output_get_2 (set `self.jumpCardNum` (- (`self.jumpCardNum`) 1)))
    (if (== _output_get_2 0)
      (if (`|EnumEquality` (`self.Card1`) "NewEnumerator0")
        (set `self.isAbility1Free` true)
        (else
          (set `self.isAbility2Free` true)))
      (`self.CardChangeEvent`))))

(fn `ClickSprintCard`
  (bind _returnvalue (`KismetMathLibrary.FFloor` (* (`self.ShieldTime`) 10.0)))
  (bind _returnvalue_2 (/ _returnvalue 10))
  (if (`self.bShieldOpen`)
    (set `self.bShieldOpen` false)
    (set `self.ShieldTime` (/ (`KismetMathLibrary.Conv_IntToDouble` _returnvalue) 10.0))
    (if (== (mod _returnvalue 10) 0)
      (bind _output_get (set `self.sprintCardNum` _returnvalue_2))
      (if (== _output_get 0)
        (set `self.bShieldOpen` false)
        (if (`|EnumEquality` (`self.Card1`) "NewEnumerator2")
          (set `self.isAbility1Free` true)
          (else
            (set `self.isAbility2Free` true)))
        (`self.CardChangeEvent`)
        (else
          (`self.CardChangeEvent` :!label _label)))
      (else
        (set `self.sprintCardNum` (+ _returnvalue_2 1))
        (goto _label)))
    (else
      (set `self.bShieldOpen` true))))

(fn `CollectBoomCard`
  (set `self.boomCardNum` (+ (`self.boomCardNum`) 1))
  (set `self.rifleGunAmmo` (`KismetMathLibrary.Clamp` (+ (`self.rifleGunAmmo`) (`self.rifleGunAmmoPerCard`)) 0 (`self.maxRifleGunAmmo`)))
  (if (== (`self.boomCardNum`) 1)
    (if (`self.isAbility1Free`)
      (set `self.isAbility1Free` false)
      (set `self.Card1` "NewEnumerator1")
      (`self.CardChangeEvent` :!label _label)
      (elif (`self.isAbility2Free`)
        (set `self.isAbility2Free` false)
        (set `self.Card2` "NewEnumerator1")
        (goto _label)))
    (else
      (`self.CardChangeEvent`))))

(fn `CollectJumpCard`
  (set `self.jumpCardNum` (`KismetMathLibrary.Clamp` (+ (`self.jumpCardNum`) 1) 0 3))
  (set `self.handGunAmmo` (`KismetMathLibrary.Clamp` (+ (`self.handGunAmmo`) (`self.handGunAmmoPerCard`)) 0 (`self.maxHandGunAmmo`)))
  (if (== (`self.jumpCardNum`) 1)
    (if (`self.isAbility1Free`)
      (set `self.isAbility1Free` false)
      (set `self.Card1` "NewEnumerator0")
      (`self.CardChangeEvent` :!label _label)
      (elif (`self.isAbility2Free`)
        (set `self.isAbility2Free` false)
        (set `self.Card2` "NewEnumerator0")
        (goto _label)))
    (else
      (`self.CardChangeEvent`))))

(fn `CollectSprintCard`
  (set `self.ShieldTime` (`KismetMathLibrary.FClamp` (+ (`self.ShieldTime`) 2.0) 0.0 6.0))
  (set `self.sprintCardNum` (`KismetMathLibrary.Clamp` (+ (`self.sprintCardNum`) 1) 0 3))
  (if (== (`self.sprintCardNum`) 1)
    (if (`self.isAbility1Free`)
      (set `self.isAbility1Free` false)
      (set `self.Card1` "NewEnumerator2")
      (`self.CardChangeEvent` :!label _label)
      (elif (`self.isAbility2Free`)
        (set `self.isAbility2Free` false)
        (set `self.Card2` "NewEnumerator2")
        (goto _label)))
    (else
      (`self.CardChangeEvent`))))

(fn `isBoomCardCollectable`
  (returns (isCollectable :type Boolean))
  (return (or (and (< (`self.boomCardNum`) 3) (or (== (`self.sprintCardNum`) 0) (== (`self.jumpCardNum`) 0))) (and (< (`self.rifleGunAmmo`) (`self.maxRifleGunAmmo`)) (> (`self.boomCardNum`) 0)))))

(fn `isJumpCardCollectable`
  (returns (isCollectable :type Boolean))
  (return (or (and (< (`self.jumpCardNum`) 3) (or (== (`self.sprintCardNum`) 0) (== (`self.boomCardNum`) 0))) (and (< (`self.handGunAmmo`) (`self.maxHandGunAmmo`)) (> (`self.jumpCardNum`) 0)))))

(fn `isSprintCardCollectable`
  (returns (isCollectable :type Boolean))
  (return (or (and (< (`self.sprintCardNum`) 3) (or (== (`self.jumpCardNum`) 0) (== (`self.boomCardNum`) 0))) (and (< (`self.ShieldTime`) 6.0) (> (`self.sprintCardNum`) 0)))))

(fn `SlideBoomCard`
  (`KismetSystemLibrary.PrintString` "Slide BoomCard")
  (bind _output_get (set `self.boomCardNum` (- (`self.boomCardNum`) 1)))
  (if (<= _output_get 0)
    (set `self.rifleGunAmmo` 0)
    (if (`|EnumEquality` (`self.Card1`) "NewEnumerator1")
      (set `self.isAbility1Free` true)
      (else
        (set `self.isAbility2Free` true)))
    (`self.CardChangeEvent`)
    (`self.Status`)
    (else
      (`self.CardChangeEvent`))))

(fn `SlideJumpCard`
  (`KismetSystemLibrary.PrintString` "Slide JumpCard")
  (bind _output_get (set `self.jumpCardNum` (+ (`self.jumpCardNum`) -1)))
  (if (== _output_get 0)
    (set `self.handGunAmmo` 0)
    (if (`|EnumEquality` (`self.Card1`) "NewEnumerator0")
      (set `self.isAbility1Free` true)
      (else
        (set `self.isAbility2Free` true)))
    (`self.CardChangeEvent`)
    (else
      (`self.CardChangeEvent`))))

(fn `SlideSprintCard`
  (set `self.ShieldTime` (`KismetMathLibrary.FClamp` (- (`self.ShieldTime`) 2.0) 0.0 6.0))
  (bind _output_get (set `self.sprintCardNum` (+ (`self.sprintCardNum`) -1)))
  (if (== _output_get 0)
    (if (`|EnumEquality` (`self.Card1`) "NewEnumerator2")
      (set `self.isAbility1Free` true)
      (else
        (set `self.isAbility2Free` true)))
    (`self.CardChangeEvent`)
    (else
      (`self.CardChangeEvent`))))

(fn `Status`
  (`KismetSystemLibrary.PrintString` (`KismetStringLibrary.Concat_StrStr` "Ability1Free:" (`KismetStringLibrary.Conv_BoolToString` (`self.isAbility1Free`)) "  Ability2Free:" (`KismetStringLibrary.Conv_BoolToString` (`self.isAbility2Free`))))
  (`KismetSystemLibrary.PrintString` (`KismetStringLibrary.Concat_StrStr` "炸弹卡数量" (`KismetStringLibrary.Conv_IntToString` (`self.boomCardNum`))))
  (`KismetSystemLibrary.PrintString` (`KismetStringLibrary.Concat_StrStr` "跳跃卡数量" (`KismetStringLibrary.Conv_IntToString` (`self.jumpCardNum`))))
  (`KismetSystemLibrary.PrintString` (`KismetStringLibrary.Concat_StrStr` "冲刺卡数量" (`KismetStringLibrary.Conv_IntToString` (`self.sprintCardNum`))))
  (`KismetSystemLibrary.PrintString` (`KismetStringLibrary.Concat_StrStr` "Jump:" (`KismetStringLibrary.Conv_BoolToString` (`self.isJumpCardCollectable`)) "Sprint:" (`KismetStringLibrary.Conv_BoolToString` (`self.isSprintCardCollectable`)) "Boom:" (`KismetStringLibrary.Conv_BoolToString` (`self.isBoomCardCollectable`))))
  (`KismetSystemLibrary.PrintString` (`KismetStringLibrary.Concat_StrStr` "手枪子弹数：" (`KismetStringLibrary.Conv_IntToString` (`self.handGunAmmo`)) "手枪子弹上限:" (`KismetStringLibrary.Conv_IntToString` (`self.maxHandGunAmmo`)) "步枪子弹数：" (`KismetStringLibrary.Conv_IntToString` (`self.rifleGunAmmo`)) "步枪子弹上限:" (`KismetStringLibrary.Conv_IntToString` (`self.maxRifleGunAmmo`)))))