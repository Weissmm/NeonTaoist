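; Base AI controller for monsters that turn and fire projectiles at the player while they sense them.
; Perception updates start looping attack and rotation timers for a sensed Player-tagged actor, and clear them otherwise.
; Attacks spawn ProjectileClass from the pawn toward the target, while rotation applies GetMonsterNewRoll.
; Rotation switches a non-movable BP_MonsterBase box to Movable, then back to Stationary if the player is standing on the monster.
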(event `self.AIPerception.OnTargetPerceptionUpdated`
  (params (Actor :type "Actor Object Reference") (Stimulus :type "AIStimulus Structure"))
  (if (and (`self.ActorHasTag` Actor "Player") (`.bSuccessfullySensed` (break `AIStimulus` Stimulus)))
    (bind _returnvalue (`KismetSystemLibrary.K2_SetTimerDelegate` (delegate `Attack Player`) (`self.AttackPeriod`) true))
    (set `self.AttackTimerHandle` _returnvalue)
    (bind _returnvalue_2 (`KismetSystemLibrary.K2_SetTimerDelegate` (delegate `MonsterRotate`) 0.05 true))
    (set `self.RotateTimerHandle` _returnvalue_2)
    (else
      (`KismetSystemLibrary.K2_ClearAndInvalidateTimerHandle` (`self.AttackTimerHandle`))
      (`KismetSystemLibrary.K2_ClearAndInvalidateTimerHandle` (`self.RotateTimerHandle`)))))

(event `MonsterRotate`
  (bind _returnvalue (`self.K2_GetPawn`))
  (bind _asbp_monster_base (cast `/Game/ThirdPerson/Blueprints/Monster/Base/BP_MonsterBase` (`self.K2_GetPawn`)))
  (bind _returnvalue_2 (`NeonTaoistAbilityCommon.GetMonsterNewRoll` (`GameplayStatics.GetPlayerPawn` 0) _returnvalue))
  (bind _boxcomponent (`NeonTaoistMonsterBase.BoxComponent` _asbp_monster_base))
  (if (`|EnumEquality` (`SceneComponent.Mobility` _boxcomponent) "Movable")
    (`self.K2_SetActorRotation` _returnvalue _returnvalue_2 false)
    (else
      (`SceneComponent.SetMobility` _boxcomponent "Movable")
      (`self.K2_SetActorRotation` _returnvalue _returnvalue_2 false)
      (bind _isplayerstandon (`self.IsPlayerStandOn`))
      (if _isplayerstandon
        (`SceneComponent.SetMobility` _boxcomponent "Stationary")))))

(event `Attack Player`
  (bind _returnvalue (`self.K2_GetPawn`))
  (bind _returnvalue_2 (`self.K2_GetActorLocation` _returnvalue))
  (`|SpawnActorFromClass` (`self.ProjectileClass`) (`KismetMathLibrary.MakeTransform` _returnvalue_2) "AlwaysSpawn" "OverrideRootScale" _returnvalue (- (`self.K2_GetActorLocation` (stale `self.AIPerception.OnTargetPerceptionUpdated` Actor)) _returnvalue_2) _returnvalue))

(fn `IsPlayerStandOn`
  (returns (IsPlayerStandOn :type Boolean))
  (bind _asbp_third_person_character (cast `/Game/ThirdPerson/Blueprints/BP_ThirdPersonCharacter` (`GameplayStatics.GetPlayerPawn` 0)))
  (bind _returnvalue (`CharacterMovementComponent.GetMovementBase` (`Character.CharacterMovement` _asbp_third_person_character)))
  (`/Engine/EditorBlueprintResources/StandardMacros.IsValid` _returnvalue
    (:`Is Valid`
      (return (== (`ActorComponent.GetOwner` _returnvalue) (`self.K2_GetPawn`))))))

(fn `UserConstructionScript`)