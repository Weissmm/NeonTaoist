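; Base monster Blueprint with a health bar, death feedback and card drops, built on the Gameplay Ability System.
; Health change events update the widget bar, whose transform is made absolute at BeginPlay to detach it from the actor's movement.
; On dying it disables box collision, plays effects and grants player energy through a negated cost GameplayEffect.
; It then spawns CardCount cards, spacing multiples along world X or Y chosen by an IsDirectionY player check.
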(event `self.ReceiveBeginPlay`
  (add `self.HealthChangeEvent` (delegate `HealthChangeEvent_Event`))
  (`self.SetWidget`)
  (add `self.OnDying` (delegate `OnDying_Event`)))

(event `OnDying_Event`
  (bind (_returnvalue_location _returnvalue_rotation) (`KismetMathLibrary.BreakTransform` (`self.GetTransform`)))
  (`PrimitiveComponent.SetCollisionEnabled` (`self.BoxComponent`) "NoCollision")
  (`GameplayStatics.SpawnEmitterAtLocation` "/Game/VFX_Pack/Particles/P_Mid_Explosion.P_Mid_Explosion" _returnvalue_location _returnvalue_rotation (0.2 0.2 0.2))
  (`NeonTaoistAbilityCommon.ApplyGEToTargetWithCallerData` self (`GameplayStatics.GetPlayerPawn` 0) "/Game/ThirdPerson/Blueprints/Abilities/Character/GE_CostEnergy.GE_CostEnergy_C" (struct :`TagName` "GE.CostEnergy") (* (`self.AddEnergy`) -1.0))
  (`GameplayStatics.PlaySound2D` "/Game/AudioResource/Sounds/UI/Sounds_Kill.Sounds_Kill" 1.0 1.0 0.0 null null)
  (if (> (`self.CardCount`) 0)
    (`self.SpawnCards`)))

(event `HealthChangeEvent_Event` :!signature `self.HealthChangeEvent`
  (params (NewHealth :type "Float (single-precision)"))
  (bind _aswbp_monster_health (cast `/Game/ThirdPerson/Blueprints/Monster/Base/WBP_MonsterHealth` (`WidgetComponent.GetWidget` (`self.Widget`))))
  (`ProgressBar.SetPercent` (`/Game/ThirdPerson/Blueprints/Monster/Base/WBP_MonsterHealth.MonsterProgressBar` _aswbp_monster_health) (/ NewHealth (`.ReturnValue` (`AbilitySystemBlueprintLibrary.GetFloatAttributeFromAbilitySystemComponent` (`self.AbilitySystem`) (struct :`AttributeName` "MaxHealth" :`Attribute` "/Script/NeonTaoist.NTAttributeSetBase:MaxHealth" :`AttributeOwner` "Class'\"/Script/NeonTaoist.NTAttributeSetBase\"'"))))))

(fn `GetCardLocation`
  (params (CardNum :type Integer))
  (returns (CardLocation :type "Vector Structure"))
  (bind (_curcardlocation_x _curcardlocation_y _curcardlocation_z) (`KismetMathLibrary.BreakVector` (`self.CurCardLocation`)))
  (bind (_curcardlocation_x_2 _curcardlocation_y_2 _curcardlocation_z_2) (`KismetMathLibrary.BreakVector` (`self.CurCardLocation`)))
  (set `self.CurCardLocation` (`self.K2_GetActorLocation`))
  (bind _returnvalue (`NeonTaoistAbilityCommon.IsDirectionY` (`GameplayStatics.GetPlayerPawn` 0)))
  (if _returnvalue
    (set `self.CurCardLocation` (`KismetMathLibrary.MakeVector` _curcardlocation_x_2 (+ (* (`self.CardDistance`) CardNum) (- _curcardlocation_y_2 (`self.CardDistance`))) _curcardlocation_z_2))
    (else
      (set `self.CurCardLocation` (`KismetMathLibrary.MakeVector` (+ (* (`self.CardDistance`) CardNum) (- _curcardlocation_x (`self.CardDistance`))) _curcardlocation_y _curcardlocation_z))))
  (return (`self.CurCardLocation`)))

(fn `SetWidget`
  (bind _widget (`self.Widget`))
  (bind _output_get (set `self.WidgetTransform` (`SceneComponent.K2_GetComponentToWorld` _widget)))
  (`SceneComponent.SetAbsolute` _widget true true true)
  (`SceneComponent.K2_SetWorldTransform` _widget _output_get false true))

(fn `SpawnCards`
  (bind (_returnvalue_roll _returnvalue_pitch _returnvalue_yaw) (`KismetMathLibrary.BreakRotator` (`self.K2_GetActorRotation`)))
  (bind _returnvalue (`self.GetTransform`))
  (if (== (`self.CardCount`) 1)
    (`|SpawnActorFromClass` (`self.CardClass`) (`KismetMathLibrary.MakeTransform` (.location _returnvalue) (`KismetMathLibrary.MakeRotator` 0.0 0.0 (.yaw (.rotation _returnvalue)))) "Undefined" "OverrideRootScale" self self)
    (else
      (for _index (range 1 (+ (`self.CardCount`) 1))
        (bind _cardlocation (`self.GetCardLocation` _index))
        (`|SpawnActorFromClass` (`self.CardClass`) (`KismetMathLibrary.MakeTransform` _cardlocation (`KismetMathLibrary.MakeRotator` 0.0 0.0 _returnvalue_yaw)) "Undefined" "OverrideRootScale" self self)))))

(fn `UserConstructionScript`)