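; Base monster projectile that flies along a local-space direction at an initial speed and damages what it hits.
; Overlapping a component tagged "Body" applies a damage GameplayEffect from the Instigator, passing Damage as the caller-set magnitude.
; For a BP_Character target, it briefly pulses IsHurting on the anim instance before calling SafeDestory.
; Non-Body overlaps go straight to SafeDestory, while a failed character or anim cast skips it.
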(event `self.ReceiveBeginPlay`
  (`ProjectileMovementComponent.SetVelocityInLocalSpace` (`self.ProjectileMovement`) (* (`KismetMathLibrary.Normal` (`self.MoveForwardDirection`)) (`self.InitSpeed`))))

(event `self.Sphere.OnComponentBeginOverlap`
  (params (OverlappedComponent :type "PrimitiveComponent Object Reference") (OtherActor :type "Actor Object Reference") (OtherComp :type "PrimitiveComponent Object Reference") (OtherBodyIndex :type Integer) (bFromSweep :type Boolean) (SweepResult :type "HitResult Structure (by ref)"))
  (if (`ActorComponent.ComponentHasTag` OtherComp "Body")
    (`NeonTaoistAbilityCommon.ApplyGEToTargetWithCallerData` (`self.Instigator`) OtherActor "/Game/ThirdPerson/Blueprints/Abilities/Character/GE_DealDamage.GE_DealDamage_C" (struct :`TagName` "GE.DamageMagnitude") (`self.Damage`))
    (bind _asbp_character (cast `/Game/Art/Frank_Platformer1/Animations/BP_Character` OtherActor))
    (bind _asabp_character (cast `/Game/Art/Frank_Platformer1/Animations/ABP_Character` (`NeonTaoistCharacter.AnimInstance` _asbp_character)))
    (set `/Game/Art/Frank_Platformer1/Animations/ABP_Character.IsHurting` true _asabp_character)
    (`KismetSystemLibrary.Delay` 0.1)
    (set `/Game/Art/Frank_Platformer1/Animations/ABP_Character.IsHurting` false _asabp_character))
  (`self.SafeDestory` 0.1))

(fn `UserConstructionScript`
  (`parent.UserConstructionScript`))