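; Gameplay ability that fires the player character's rifle.
; On activation it casts player pawn 0 to BP_Character and spawns a BP_RifleGunBullet at the Robot component's position plus ShootOffset in character space.
; It plays the rifle sound and turns on a muzzle flash through the character's Shooting Niagara component, switching it off and ending after a short delay.
; A separate ShootEffect helper is not called here.
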(event `self.K2_ActivateAbility`
  (bind _asbp_character (cast `/Game/Art/Frank_Platformer1/Animations/BP_Character` (`GameplayStatics.GetPlayerPawn` 0)))
  (bind _returnvalue (`Actor.GetTransform` _asbp_character))
  (`|SpawnActorFromClass` "/Game/ThirdPerson/Blueprints/Gameplay/Projectile/BP_RifleGunBullet.BP_RifleGunBullet_C" (`KismetMathLibrary.MakeTransform` (`KismetMathLibrary.TransformLocation` _returnvalue (+ (`KismetMathLibrary.InverseTransformLocation` _returnvalue (`SceneComponent.K2_GetComponentLocation` (`/Game/Art/Frank_Platformer1/Animations/BP_Character.Robot` _asbp_character))) (`self.ShootOffset`)))) "AlwaysSpawn" "OverrideRootScale" null null)
  (`GameplayStatics.PlaySound2D` "/Game/AudioResource/Sounds/Card/Sound_Rifle.Sound_Rifle" 1.0 1.0 0.0 null null)
  (bind _shooting (`/Game/Art/Frank_Platformer1/Animations/BP_Character.Shooting` _asbp_character))
  (`NiagaraComponent.SetAsset` _shooting "/Game/Muzzle_Flash/MuzzleFlashes/MuzzleFlash_16/NS_MuzzleFlash_16.NS_MuzzleFlash_16" true)
  (`ActorComponent.SetActive` _shooting true false)
  (`|ExecutionSequence`
    (:`then_0`
      (`KismetSystemLibrary.Delay` 0.2)
      (`ActorComponent.SetActive` (`/Game/Art/Frank_Platformer1/Animations/BP_Character.Shooting` _asbp_character) false false)
      (`self.K2_EndAbility`))))

(fn `ShootEffect`
  (params (Location :type "Vector Structure"))
  (`NiagaraFunctionLibrary.SpawnSystemAttached` "/Game/Muzzle_Flash/MuzzleFlashes/MuzzleFlash_25/NS_MuzzleFlash_25.NS_MuzzleFlash_25" null "None" Location (struct) "KeepRelativeOffset"))