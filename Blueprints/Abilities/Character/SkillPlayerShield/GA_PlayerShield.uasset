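; Gameplay ability that gives the player character a temporary shield.
; On activation it reads ShieldTime from the character's BPCCharacterCardList and cancels if that is not positive.
; Otherwise it spawns BP_PlayerShiled at the owner's location with that keep time and attaches it to the owner.
; The ability stays active until the shield actor is destroyed, then ends through the OnDestroyed binding.
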(event `self.K2_ActivateAbility`
  (bind _returnvalue (`self.GetOwningActorFromActorInfo`))
  (`self.GetKeepTime`)
  (if (> (`self.Keep Time`) 0.0)
    (bind _returnvalue_2 (`|SpawnActorFromClass` "/Game/ThirdPerson/Blueprints/Abilities/Character/SkillPlayerShield/BP_PlayerShiled.BP_PlayerShiled_C" (`KismetMathLibrary.MakeTransform` (`Actor.K2_GetActorLocation` _returnvalue)) "Undefined" "OverrideRootScale" _returnvalue (`self.Keep Time`) null))
    (bind _output_get (set `self.SpawnedShield` _returnvalue_2))
    (`Actor.K2_AttachToActor` _output_get (`self.GetOwningActorFromActorInfo`) "None" "KeepWorld" "KeepWorld" "KeepWorld" true)
    (add `Actor.OnDestroyed` (`self.SpawnedShield`) (delegate `ShiledDestroyed`))
    (else
      (`self.K2_CancelAbility`))))

(event `ShiledDestroyed`
  (params (DestroyedActor :type "Actor Object Reference"))
  (`self.K2_EndAbility`))

(fn `GetKeepTime`
  (bind _asbp_third_person_character (cast `/Game/ThirdPerson/Blueprints/BP_ThirdPersonCharacter` (`self.GetOwningActorFromActorInfo`)))
  (set `self.Keep Time` (`/Game/ThirdPerson/Blueprints/Characters/BPC_CharacterCardList.ShieldTime` (`/Game/ThirdPerson/Blueprints/BP_ThirdPersonCharacter.BPC_CharacterCardList` _asbp_third_person_character))))