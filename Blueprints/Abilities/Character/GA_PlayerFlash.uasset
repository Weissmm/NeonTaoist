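; GA_PlayerFlash is a Gameplay Ability that performs the player character's flash, a short teleport.
; On activation it records the larger of the signed X and Y velocity components, plays a sped-up dash montage and triggers the character's flash effect.
; When the montage completes, it teleports by the flash axis distance, sets post-flash velocity from the recorded speed, base speed and ratio, plays sounds and ends the ability.
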(event `self.K2_ActivateAbility`
  (bind _neon_taoist_character (`self.Neon Taoist Character`))
  (bind _asbp_character (cast `/Game/Art/Frank_Platformer1/Animations/BP_Character` (`self.GetOwningActorFromActorInfo`)))
  (set `self.Neon Taoist Character` _asbp_character)
  (`|ExecutionSequence`
    (:`then_0`
      (`self.GetInitVelocity`)
      (`AbilityTask_PlayMontageAndWait.CreatePlayMontageAndWaitProxy` "None" "/Game/Art/Frank_Platformer1/Animations/02_Demo_215Anim/02_Moving_InPlace_RootMotion/Frank_Dash.Frank_Dash" 5.0
        (:`OnCompleted`
          (`NeonTaoistAbilityCommon.TryTeleportTo` _neon_taoist_character (`self.FlashAxisDistance`) (`Actor.K2_GetActorRotation` _neon_taoist_character))
          (`NeonTaoistAbilityCommon.SetVelocityAfterFlash` _neon_taoist_character (`self.BaseSpeed`) (`self.PlayerSpeed`) (`self.VelocityRatio`))
          (`GameplayStatics.PlaySound2D` "/Engine/VREditor/Sounds/UI/Dockable_Window_Open.Dockable_Window_Open" 1.0 1.0 0.0 null null)
          (`self.K2_EndAbility`)
          (`GameplayStatics.PlaySound2D` "/Engine/EditorSounds/GamePreview/EjectFromPlayer.EjectFromPlayer" 1.0 1.0 0.0 null null))))
    (:`then_1`
      (`/Game/Art/Frank_Platformer1/Animations/BP_Character.Effect_Flash` _asbp_character))))

(fn `GetInitVelocity`
  (bind (_velocity_x _velocity_y) (`KismetMathLibrary.BreakVector` (`MovementComponent.Velocity` (`Pawn.GetMovementComponent` (`self.Neon Taoist Character`)))))
  (set `self.PlayerSpeed` (`KismetMathLibrary.FMax` _velocity_x _velocity_y)))