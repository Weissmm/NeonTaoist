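; Gameplay ability that dashes player pawn 0 forward by SprintDistance, with sound, montage and a brief Niagara burst.
; On activation it sets sprint state, computes the target and disables input.
; A looping timer moves the pawn by swept constant-speed interpolation until blocked or arrived.
; It then restores input, clears sprint via a BP_ThirdPersonCharacter cast (BP_Character at start), starts looping FOV-nudge timers and ends the ability.
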(event `self.K2_ActivateAbility`
  (`GameplayStatics.PlaySound2D` "/Engine/VREditor/Sounds/VR_teleport.VR_teleport" 1.0 1.0 0.0 null null)
  ;[1 1 1] For Dependency Effect Component
  (bind _asbp_character (cast `/Game/Art/Frank_Platformer1/Animations/BP_Character` (`GameplayStatics.GetPlayerPawn` 0)))
  (`/Game/ThirdPerson/Blueprints/BP_ThirdPersonCharacter.SprintState` _asbp_character true)
  (`AbilityTask_PlayMontageAndWait.CreatePlayMontageAndWaitProxy` "None" "/Game/Art/Frank_Platformer1/Animations/02_Demo_215Anim/02_Moving_InPlace_RootMotion/Frank_Dash.Frank_Dash"
    (:`then`
      (bind _dash (`/Game/Art/Frank_Platformer1/Animations/BP_Character.Dash` _asbp_character))
      ;[1 1 1] FX Effect
      (`NiagaraComponent.SetAsset` _dash "/Game/Muzzle_Flash/MuzzleFlashes/MuzzleFlash_10/NS_MuzzleFlash_10.NS_MuzzleFlash_10" true)
      (`ActorComponent.SetActive` _dash true false)
      (`KismetSystemLibrary.Delay` 0.02)
      (`ActorComponent.SetActive` _dash false false)
      (`self.GetTargetLocation`)
      (`Actor.DisableInput` (`GameplayStatics.GetPlayerPawn` 0) (`GameplayStatics.GetPlayerController` 0))
      (bind _returnvalue (`KismetSystemLibrary.K2_SetTimerDelegate` (`|CreateDelegate` :!event `UpdatePlayerPostion`) 0.01 true)))))

(event `UpdatePlayerPostion`
  (bind _returnvalue (`GameplayStatics.GetPlayerPawn` 0))
  (bind _returnvalue_2 (`GameplayStatics.GetPlayerPawn` 0))
  (bind _returnvalue_3 (`Actor.K2_GetActorLocation` (`GameplayStatics.GetPlayerPawn` 0)))
  (bind _output_get (set `self.New Location` (`KismetMathLibrary.VInterpTo_Constant` (`Actor.K2_GetActorLocation` _returnvalue) (`self.TargetLocation`) 0.01 (`self.SprintSpeed`))))
  (`Actor.K2_SetActorLocation` _returnvalue _output_get true false)
  (if (or (!= (`self.New Location`) _returnvalue_3 :`ErrorTolerance` 2.0) (== _returnvalue_3 (`self.TargetLocation`) :`ErrorTolerance` 2.0))
    (`self.MontageStop` -1.0)
    (`Actor.EnableInput` (`GameplayStatics.GetPlayerPawn` 0) (`GameplayStatics.GetPlayerController` 0))
    (`KismetSystemLibrary.K2_ClearAndInvalidateTimerHandle` (stale `self.K2_ActivateAbility` _returnvalue))
    (bind _asbp_third_person_character (cast `/Game/ThirdPerson/Blueprints/BP_ThirdPersonCharacter` _returnvalue_2))
    (`/Game/ThirdPerson/Blueprints/BP_ThirdPersonCharacter.SprintState` _asbp_third_person_character false)
    (bind _asbp_third_person_character_2 (cast `/Game/ThirdPerson/Blueprints/BP_ThirdPersonCharacter` _returnvalue_2))
    (`|ExecutionSequence`
      (:`then_1`
        (`KismetSystemLibrary.K2_SetTimerDelegate` (delegate `SetCameraScale`) 0.02 true)
        (`KismetSystemLibrary.Delay` 0.1)
        (`KismetSystemLibrary.K2_SetTimerDelegate` (delegate `SetCameraScale1`) 0.02 true)
        (`KismetSystemLibrary.Delay` 0.1)
        (`self.K2_EndAbility`)))))

(event `SetCameraScale`
  (set `self.CameraAlpha` (`KismetMathLibrary.FClamp` (+ (`self.CameraAlpha`) 0.2)))
  (`CameraComponent.SetFieldOfView` (`NeonTaoistCharacter.SideViewCameraComponent` (stale `UpdatePlayerPostion` _asbp_third_person_character_2)) (`KismetMathLibrary.Lerp` 100.0 99.0 (`self.CameraAlpha`))))

(event `SetCameraScale1`
  (set `self.CameraAlpha` (`KismetMathLibrary.FClamp` (+ (`self.CameraAlpha`) 0.2)))
  (`CameraComponent.SetFieldOfView` (`NeonTaoistCharacter.SideViewCameraComponent` (stale `UpdatePlayerPostion` _asbp_third_person_character_2)) (`KismetMathLibrary.Lerp` 99.0 100.0 (`self.CameraAlpha`))))

(fn `GetTargetLocation`
  (locals (NewLocalVar_0 :type "Vector Structure" :default (0.0 0.0 0.0)))
  (bind _returnvalue (`GameplayStatics.GetPlayerPawn` 0))
  (bind _returnvalue_2 (`NeonTaoistAbilityCommon.GetForwardDirection` _returnvalue))
  (set `self.TargetLocation` (+ (`Actor.K2_GetActorLocation` _returnvalue) (* (`KismetMathLibrary.Normal` _returnvalue_2) (`self.SprintDistance`)))))