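; GA_Shoot is a Gameplay Ability that fires one handgun shot from the player's BP_Character.
; It spawns BP_HandGunBullet at ShootOffset from the Robot component, calculated in the character's local space, with the player as owner and instigator.
; It plays a 2D pistol sound and briefly activates a muzzle flash on the Shooting Niagara component before ending.
; The character comes from player pawn 0 rather than the ability's avatar.
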(event `self.K2_ActivateAbility`
  (bind _returnvalue (`GameplayStatics.GetPlayerPawn` 0))
  (bind _asbp_character (cast `/Game/Art/Frank_Platformer1/Animations/BP_Character` _returnvalue))
  (bind _returnvalue_2 (`Actor.GetTransform` _asbp_character))
  (`|SpawnActorFromClass` "/Game/ThirdPerson/Blueprints/Gameplay/Projectile/BP_HandGunBullet.BP_HandGunBullet_C" (`KismetMathLibrary.MakeTransform` (`KismetMathLibrary.TransformLocation` _returnvalue_2 (+ (`KismetMathLibrary.InverseTransformLocation` _returnvalue_2 (`SceneComponent.K2_GetComponentLocation` (`/Game/Art/Frank_Platformer1/Animations/BP_Character.Robot` _asbp_character))) (`self.ShootOffset`)))) "AlwaysSpawn" "OverrideRootScale" _returnvalue _returnvalue)
  (`GameplayStatics.PlaySound2D` "/Game/AudioResource/Sounds/Card/Sound_Pistol.Sound_Pistol" 1.0 1.0 0.0 null null)
  (bind _shooting (`/Game/Art/Frank_Platformer1/Animations/BP_Character.Shooting` _asbp_character))
  (`NiagaraComponent.SetAsset` _shooting "/Game/Muzzle_Flash/MuzzleFlashes/MuzzleFlash_01/NS_MuzzleFlash_1.NS_MuzzleFlash_1" true)
  (`ActorComponent.SetActive` _shooting true false)
  (`KismetSystemLibrary.Delay` 0.2)
  (`ActorComponent.SetActive` (`/Game/Art/Frank_Platformer1/Animations/BP_Character.Shooting` _asbp_character) false false)
  (`self.K2_EndAbility`))