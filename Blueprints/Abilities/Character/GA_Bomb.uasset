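; Gameplay ability that makes the player character throw a bomb along its BombRotation.
; On activation it caches that direction and flips the pawn's yaw 180 degrees if it doesn't already match.
; It starts a throw montage, then after a short delay spawns BP_Bomb at an offset from the pawn and sets its projectile velocity.
; The ability ends right after the launch, without waiting for the montage, and plays a sound.
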(event `self.K2_ActivateAbility`
  (`self.GetBombDirection`)
  (`self.ChangePlayerRotation`)
  (bind _asynctaskproxy (`AbilityTask_PlayMontageAndWait.CreatePlayMontageAndWaitProxy` "None" "/Game/Art/Frank_Platformer1/Animations/02_Demo_215Anim/14_Weapon_Atk/Frank_Platformer_ATK_Rock_Montage.Frank_Platformer_ATK_Rock_Montage")
    (:`then`
      (`GameplayTask_WaitDelay.TaskWaitDelay` _asynctaskproxy 0.3
        (:`OnFinish`
          (bind _returnvalue (`|SpawnActorFromClass` "/Game/ThirdPerson/Blueprints/Gameplay/Projectile/BP_Bomb.BP_Bomb_C" (`KismetMathLibrary.MakeTransform` (+ (`Actor.K2_GetActorLocation` (`GameplayStatics.GetPlayerPawn` 0)) (`self.SpawnOffset`))) "Undefined" "OverrideRootScale" null null))
          (set `MovementComponent.Velocity` (* (`self.TargetDirection`) (`/Game/ThirdPerson/Blueprints/Gameplay/Projectile/BP_ProjectileBase.Speed` _returnvalue)) (`/Game/ThirdPerson/Blueprints/Gameplay/Projectile/BP_ProjectileBase.ProjectileMovement` _returnvalue))
          (`self.K2_EndAbility`)
          (`GameplayStatics.PlaySound2D` "/Engine/VREditor/Sounds/UI/Camera_Shutter.Camera_Shutter" 1.0 1.0 0.0 null null))))))

(fn `ChangePlayerRotation`
  (bind _returnvalue (`GameplayStatics.GetPlayerPawn` 0))
  (bind _returnvalue_2 (`GameplayStatics.GetPlayerPawn` 0))
  (bind (_returnvalue_roll _returnvalue_pitch _returnvalue_yaw) (`KismetMathLibrary.BreakRotator` (`Actor.K2_GetActorRotation` _returnvalue)))
  (bind (_returnvalue_roll_2 _returnvalue_pitch_2 _returnvalue_yaw_2) (`KismetMathLibrary.BreakRotator` (`Actor.K2_GetActorRotation` _returnvalue_2)))
  (bind _asneon_taoist_character (cast `NeonTaoistCharacter` _returnvalue_2))
  (bind (_bombrotation_roll _bombrotation_pitch _bombrotation_yaw) (`KismetMathLibrary.BreakRotator` (`NeonTaoistCharacter.BombRotation` _asneon_taoist_character)))
  (if (not (`KismetMathLibrary.NearlyEqual_FloatFloat` _bombrotation_yaw _returnvalue_yaw_2 1.0))
    (`Actor.K2_SetActorRotation` _returnvalue (`KismetMathLibrary.MakeRotator` _returnvalue_roll _returnvalue_pitch (- _returnvalue_yaw 180.0)) false)))

(fn `GetBombDirection`
  (bind _asneon_taoist_character (cast `NeonTaoistCharacter` (`GameplayStatics.GetPlayerPawn` 0)))
  (set `self.TargetDirection` (`KismetMathLibrary.GetForwardVector` (`NeonTaoistCharacter.BombRotation` _asneon_taoist_character))))